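; Pac-Man character Blueprint whose only active logic is toggling the pause menu from the Pause input action.
; Each press creates and stores a pause screen widget if PauseAction is valid, then branches on the game's paused state.
; Pausing shows the stored menu, cursor and Game-and-UI input; unpausing calls remove on that stored reference, which may be newly created, and restores game-only input.
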(event `InputAction|Pause`
  (params (Key :type "Key Structure"))
  (bind _returnvalue (`GameplayStatics.GetPlayerController` 0))
  (bind _puase_menu_ref (`self.Puase Menu ref`))
  (:`Pressed`
    (`/Engine/EditorBlueprintResources/StandardMacros.IsValid` (`self.PauseAction`)
      (:`Is Valid`
        (bind _returnvalue_2 (`|CreateWidget` "/Game/UI/Gameplay/WBP_PauseScreen.WBP_PauseScreen_C"))
        (set `self.Puase Menu ref` _returnvalue_2))
      (:`Is Not Valid`
        _))
    (if (`GameplayStatics.IsGamePaused`)
      (`Widget.RemoveFromParent` _puase_menu_ref)
      (`GameplayStatics.SetGamePaused` false)
      (set `PlayerController.bShowMouseCursor` false _returnvalue)
      (`WidgetBlueprintLibrary.SetInputMode_GameOnly` _returnvalue)
      (else
        (`UserWidget.AddToViewport` _puase_menu_ref 0)
        (`GameplayStatics.SetGamePaused` true)
        (set `PlayerController.bShowMouseCursor` true _returnvalue)
        (`WidgetBlueprintLibrary.SetInputMode_GameAndUIEx` _returnvalue _puase_menu_ref "LockInFullscreen" false)))))

(event `self.ReceiveActorBeginOverlap`
  (params (OtherActor :type "Actor Object Reference")))

(fn `UserConstructionScript`)